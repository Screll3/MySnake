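; BP_SnakeElementBase is a snake segment Blueprint that colors its mesh according to whether it is the first or a body element.
; It extends the parent's SetFirstElementType and SetBodyElementType events, calling each parent version before writing MainColor to the materials' "Color" vector parameter.
; The first element gets a brightened MainColor to stand out, while body elements use it unchanged.
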(event `self.SetFirstElementType`
  (`parent.SetFirstElementType`)
  (`MeshComponent.SetVectorParameterValueOnMaterials` (`self.MeshComponent`) "Color" (`KismetMathLibrary.MakeVector` (* (.x (`self.MainColor`)) 1.3) (* (.y (`self.MainColor`)) 1.3) (* (.z (`self.MainColor`)) 1.3))))

(event `self.SetBodyElementType`
  (`parent.SetBodyElementType`)
  (`MeshComponent.SetVectorParameterValueOnMaterials` (`self.MeshComponent`) "Color" (`self.MainColor`)))

(fn `UserConstructionScript`)